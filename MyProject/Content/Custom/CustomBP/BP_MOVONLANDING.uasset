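; Platform-style actor whose static mesh shifts when NewMainCharacter enters its Box trigger and moves the opposite way when the character leaves.
; Begin and end overlap each restart their own timeline, whose MoveSlowly curve lerps the mesh toward plus or minus VerticalMovement.
; Each update lerps from the current location rather than a stored start, so movement accumulates per frame and total travel is not fixed to VerticalMovement.
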(event `self.ReceiveActorBeginOverlap`
  (params (OtherActor :type "Actor Object Reference")))

(event `self.Box.OnComponentBeginOverlap`
  (params (OverlappedComponent :type "PrimitiveComponent Object Reference") (OtherActor :type "Actor Object Reference") (OtherComp :type "PrimitiveComponent Object Reference") (OtherBodyIndex :type Integer) (bFromSweep :type Boolean) (SweepResult :type "HitResult Structure (by ref)"))
  (bind _staticmeshcomponent (`self.StaticMeshComponent`))
  (bind _returnvalue (`SceneComponent.K2_GetComponentLocation` _staticmeshcomponent))
  (cast `/Game/Custom/NewMainCharacter` OtherActor)
  (bind (_direction _moveslowly) (`Timeline|Timeline_0` :!via `PlayFromStart`)
    (:`Update`
      (`SceneComponent.K2_SetWorldLocation` _staticmeshcomponent (`KismetMathLibrary.VLerp` _returnvalue (+ _returnvalue (`self.VerticalMovement`)) _moveslowly) false false))))

(event `self.Box.OnComponentEndOverlap`
  (params (OverlappedComponent :type "PrimitiveComponent Object Reference") (OtherActor :type "Actor Object Reference") (OtherComp :type "PrimitiveComponent Object Reference") (OtherBodyIndex :type Integer))
  (bind (_verticalmovement_x _verticalmovement_y _verticalmovement_z) (`KismetMathLibrary.BreakVector` (`self.VerticalMovement`)))
  (bind _staticmeshcomponent (`self.StaticMeshComponent`))
  (bind _returnvalue (`SceneComponent.K2_GetComponentLocation` _staticmeshcomponent))
  (cast `/Game/Custom/NewMainCharacter` OtherActor)
  (bind (_direction _moveslowly) (`Timeline|Timeline_1` :!via `PlayFromStart`)
    (:`Update`
      (`SceneComponent.K2_SetWorldLocation` _staticmeshcomponent (`KismetMathLibrary.VLerp` _returnvalue (+ _returnvalue (`KismetMathLibrary.MakeVector` (* -1 _verticalmovement_x) (* -1 _verticalmovement_y) (* -1 _verticalmovement_z))) _moveslowly) false false))))

(fn `UserConstructionScript`)