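; BP_TopWall_Des is a destructible top wall piece that shakes and breaks apart when a NewMainCharacter overlaps it.
; The overlap plays a timeline that jitters the DestructibleComponent with random sine offsets, then applies massive damage with an impulse and disables its collision.
; Tick keeps calling Play on a second timeline, which lerps the component between the actor location and a slight fixed Y/Z offset from it.
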(event `self.ReceiveActorBeginOverlap`
  (params (OtherActor :type "Actor Object Reference"))
  (bind _destructiblecomponent (`self.DestructibleComponent`))
  (cast `/Game/Custom/NewMainCharacter` OtherActor)
  (`Timeline|Timeline_0`
    (:`Update`
      (`SceneComponent.K2_AddLocalOffset` (`self.DestructibleComponent`) (`KismetMathLibrary.MakeVector` (`KismetMathLibrary.Sin` (`KismetMathLibrary.RandomFloatInRange` -1.0 1.0)) (`KismetMathLibrary.Sin` (`KismetMathLibrary.RandomFloatInRange` -1.0 1.0)) (`KismetMathLibrary.Sin` (`KismetMathLibrary.RandomFloatInRange` -1.0 1.0))) false false))
    (:`Finished`
      (`DestructibleComponent.ApplyDamage` _destructiblecomponent 100000.0 (`self.K2_GetActorLocation`) (1.0 1.0 1.0) 10000.0)
      (`PrimitiveComponent.SetCollisionEnabled` _destructiblecomponent "NoCollision"))))

(event `self.ReceiveTick`
  (params (DeltaSeconds :type "Float (single-precision)"))
  (bind _returnvalue (`self.K2_GetActorLocation`))
  (bind (_direction _newtrack_0) (`Timeline|Timeline_1`)
    (:`Update`
      (`SceneComponent.K2_SetWorldLocation` (`self.DestructibleComponent`) (`KismetMathLibrary.VLerp` _returnvalue (+ _returnvalue (`KismetMathLibrary.MakeVector` 0.0 (* (`KismetMathLibrary.Sin` 1.0) 0.3) (* (`KismetMathLibrary.Sin` 1.0) -0.2))) _newtrack_0) false false))))

(fn `UserConstructionScript`)