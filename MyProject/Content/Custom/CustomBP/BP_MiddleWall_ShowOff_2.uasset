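; BP_MiddleWall_ShowOff_2 is a wall actor that shakes and then shatters automatically when play begins.
; A Shake timeline jitters the DestructibleComponent each update with the sine of random per-axis values, so the offsets accumulate as a random walk.
; When the timeline finishes, massive damage with an impulse at the actor's location fractures the component, and its collision is disabled.
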(event `self.ReceiveBeginPlay`
  (bind _destructiblecomponent (`self.DestructibleComponent`))
  (`Timeline|Shake`
    (:`Update`
      (`SceneComponent.K2_AddLocalOffset` (`self.DestructibleComponent`) (`KismetMathLibrary.MakeVector` (`KismetMathLibrary.Sin` (`KismetMathLibrary.RandomFloatInRange` -1.0 1.0)) (`KismetMathLibrary.Sin` (`KismetMathLibrary.RandomFloatInRange` -1.0 1.0)) (`KismetMathLibrary.Sin` (`KismetMathLibrary.RandomFloatInRange` -1.0 1.0))) false false))
    (:`Finished`
      (`DestructibleComponent.ApplyDamage` _destructiblecomponent 100000.0 (`self.K2_GetActorLocation`) (1.0 1.0 1.0) 10000.0)
      (`PrimitiveComponent.SetCollisionEnabled` _destructiblecomponent "NoCollision"))))

(fn `UserConstructionScript`)