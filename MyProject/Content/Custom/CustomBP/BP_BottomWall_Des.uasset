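; BP_BottomWall_Des is a destructible wall that shakes and breaks apart when the main character overlaps it.
; The overlap starts a Shake timeline that jitters the root with random sine offsets, then applies huge damage to the destructible mesh and disables its collision.
; Separately, Tick calls Play on the Tryagain timeline, whose updates nudge the root along positive Y and Z through a lerp with constant sine-derived offsets.
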(event `self.ReceiveActorBeginOverlap`
  (params (OtherActor :type "Actor Object Reference"))
  (bind _obj_bottom_wall_dm (`self.OBJ_BOTTOM_WALL_DM`))
  (cast `/Game/Custom/NewMainCharacter` OtherActor)
  (`Timeline|Shake`
    (:`Update`
      (`SceneComponent.K2_AddLocalOffset` (`self.DefaultSceneRoot`) (`KismetMathLibrary.MakeVector` (`KismetMathLibrary.Sin` (`KismetMathLibrary.RandomFloatInRange` -1.0 1.0)) (`KismetMathLibrary.Sin` (`KismetMathLibrary.RandomFloatInRange` -1.0 1.0)) (`KismetMathLibrary.Sin` (`KismetMathLibrary.RandomFloatInRange` -1.0 1.0))) false false))
    (:`Finished`
      (`DestructibleComponent.ApplyDamage` _obj_bottom_wall_dm 100000.0 (`self.K2_GetActorLocation`) (1.0 1.0 1.0) 10000.0)
      (`PrimitiveComponent.SetCollisionEnabled` _obj_bottom_wall_dm "NoCollision")
      (set `self.FakeVar` false))))

(event `self.ReceiveTick`
  (params (DeltaSeconds :type "Float (single-precision)"))
  (bind _returnvalue (`self.K2_GetActorLocation`))
  (bind (_direction _newtrack_0) (`Timeline|Tryagain`)
    (:`Update`
      (`SceneComponent.K2_SetWorldLocation` (`self.DefaultSceneRoot`) (`KismetMathLibrary.VLerp` _returnvalue (+ _returnvalue (`KismetMathLibrary.MakeVector` 0.0 (* (`KismetMathLibrary.Sin` 1.0) 0.3) (* (`KismetMathLibrary.Sin` 1.0) 0.2))) _newtrack_0) false false))))

(fn `UserConstructionScript`)