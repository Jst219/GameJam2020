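; BP_KillFloor is a kill floor that respawns the player character at a Checkpoint location.
; Overlapping the Floor component sets DeathTouch on a NewMainCharacter.
; Tick polls that flag on player zero, then destroys the character, spawns and possesses a replacement, and clears the flag.
; A DoOnce with no reset gates the respawn, so it runs only once per kill floor instance.
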(event `self.ReceiveTick`
  (params (DeltaSeconds :type "Float (single-precision)"))
  (bind _asnew_main_character (cast `/Game/Custom/NewMainCharacter` (`GameplayStatics.GetPlayerCharacter` 0)))
  (if (`/Game/Custom/NewMainCharacter.DeathTouch` _asnew_main_character)
    (`/Engine/EditorBlueprintResources/StandardMacros.DoOnce` false
      (:`Completed`
        (`self.K2_DestroyActor` _asnew_main_character)
        (bind _returnvalue (`|SpawnActorFromClass` "/Game/Custom/NewMainCharacter.NewMainCharacter_C" (`KismetMathLibrary.MakeTransform` (`self.Checkpoint`)) "Undefined" "OverrideRootScale" null null))
        (`Controller.Possess` (`GameplayStatics.GetPlayerController` 0) _returnvalue)
        (set `/Game/Custom/NewMainCharacter.DeathTouch` false _returnvalue)))))

(event `self.Floor.OnComponentBeginOverlap`
  (params (OverlappedComponent :type "PrimitiveComponent Object Reference") (OtherActor :type "Actor Object Reference") (OtherComp :type "PrimitiveComponent Object Reference") (OtherBodyIndex :type Integer) (bFromSweep :type Boolean) (SweepResult :type "HitResult Structure (by ref)"))
  (bind _asnew_main_character (cast `/Game/Custom/NewMainCharacter` OtherActor))
  (set `/Game/Custom/NewMainCharacter.DeathTouch` true _asnew_main_character))

(fn `UserConstructionScript`)