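; BP_upAndDown is a moving-mesh actor that travels out along a configurable XYZ offset and back, starting on BeginPlay.
; Two timelines alternate through GoDown and GoingUp events, with an optional delay after each leg.
; Each update lerps from the mesh's current world location rather than a cached origin, so movement accumulates per frame.
; With the delay enabled, nothing follows the return-leg delay, so only the no-delay path loops.
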(event `self.ReceiveBeginPlay`
  (bind _staticmeshcomponent (`self.StaticMeshComponent`))
  (bind _returnvalue (`SceneComponent.K2_GetComponentLocation` _staticmeshcomponent))
  (bind (_direction _goup) (`Timeline|GoUp` :!via `PlayFromStart` :!label _label)
    (:`Update`
      (`SceneComponent.K2_SetWorldLocation` _staticmeshcomponent (`KismetMathLibrary.VLerp` _returnvalue (+ _returnvalue (`KismetMathLibrary.MakeVector` (`self.XMovement`) (`self.YMovement`) (`self.ZMovement`))) _goup) false false))
    (:`Finished`
      (if (`self.WantADelay`)
        (`KismetSystemLibrary.Delay` (`KismetMathLibrary.Conv_IntToDouble` (`self.DelayLength`))))
      (`self.GoDown`))))

(event `GoingUp`
  (goto _label :!via `PlayFromStart`))

(event `GoDown`
  (bind _staticmeshcomponent (`self.StaticMeshComponent`))
  (bind _returnvalue (`SceneComponent.K2_GetComponentLocation` _staticmeshcomponent))
  (bind (_direction _goup) (`Timeline|Timeline_0` :!via `PlayFromStart`)
    (:`Update`
      (`SceneComponent.K2_SetWorldLocation` _staticmeshcomponent (`KismetMathLibrary.VLerp` _returnvalue (+ _returnvalue (`KismetMathLibrary.MakeVector` (* -1 (`self.XMovement`)) (* -1 (`self.YMovement`)) (* -1 (`self.ZMovement`)))) _goup) false false))
    (:`Finished`
      (if (`self.WantADelay`)
        (`KismetSystemLibrary.Delay` (`KismetMathLibrary.Conv_IntToDouble` (`self.DelayLength`)))
        (else
          (`self.GoingUp`))))))

(fn `UserConstructionScript`)